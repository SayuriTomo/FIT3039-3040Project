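; Inspection actor that displays a collectible's mesh alongside a widget showing its name and description.
; Display sets the mesh, adds the widget to the viewport and moves input from the player to this actor.
; Left-mouse drag rotates the mesh, while the wheel zooms by changing the SceneCaptureComponent2D's FOV within limits.
; The GetCollection action restores player input, removes the widget and destroys the actor.
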(event `/Game/FIT3039-3040Project/Blueprints/BP_CollectionInterface.Display`
  (params (Player :type "/Game/FirstPerson/Blueprints/BP_FirstPersonCharacter Object Reference") (ItemToFoucs :type "StaticMesh Object Reference") (CollectionName :type Text) (CollectionDescription :type Text))
  (bind _returnvalue (`GameplayStatics.GetPlayerController` 0))
  ;[1 1 1] Display
  (set `self.Player` Player)
  (`StaticMeshComponent.SetStaticMesh` (`self.ItemToFoucs`) ItemToFoucs)
  (bind _returnvalue_2 (`|CreateWidget` "/Game/FIT3039-3040Project/UI/CollectionDisplay_UI.CollectionDisplay_UI_C" null CollectionName CollectionDescription))
  (bind _output_get (set `self.DisplayWidget` _returnvalue_2))
  (`UserWidget.AddToViewport` _output_get 0)
  (`self.DisableInput` (`self.Player`) _returnvalue)
  (`self.EnableInput` _returnvalue))

(event `InputAction|GetCollection`
  (params (Key :type "Key Structure"))
  (bind _returnvalue (`GameplayStatics.GetPlayerController` 0))
  ;[1 1 1] Display
  (:`Pressed`
    (`self.DisableInput` _returnvalue)
    (`self.EnableInput` (`self.Player`) _returnvalue)
    (`Widget.RemoveFromParent` (`self.DisplayWidget`))
    (set `self.DisplayWidget` null)
    (`self.K2_DestroyActor`)))

(event `Key|LeftMouseButton`
  (params (Key :type "Key Structure"))
  ;[1 1 1] Rotate
  (:`Pressed`
    (set `self.CanRotate` true))
  (:`Released`
    (set `self.CanRotate` false)))

(event `InputAxisKey|MouseX`
  (params (AxisValue :type "Float (single-precision)"))
  ;[1 1 1] Rotate
  (if (`self.CanRotate`)
    (`SceneComponent.K2_SetWorldRotation` (`self.ItemToFoucs`) (`KismetMathLibrary.ComposeRotators` (`SceneComponent.K2_GetComponentRotation` (`self.ItemToFoucs`)) (`KismetMathLibrary.MakeRotator` 0.0 0.0 (* AxisValue -3.0))) false false)))

(event `InputAxisKey|MouseY`
  (params (AxisValue :type "Float (single-precision)"))
  ;[1 1 1] Rotate
  (if (`self.CanRotate`)
    (`SceneComponent.K2_SetWorldRotation` (`self.ItemToFoucs`) (`KismetMathLibrary.ComposeRotators` (`SceneComponent.K2_GetComponentRotation` (`self.ItemToFoucs`)) (`KismetMathLibrary.MakeRotator` (* AxisValue -3.0))) false false)))

(event `Key|MouseScrollUp`
  (params (Key :type "Key Structure"))
  (bind _scenecapturecomponent2d (`self.SceneCaptureComponent2D`))
  ;[1 1 1] Scale
  (:`Pressed`
    (set `SceneCaptureComponent2D.FOVAngle` (`KismetMathLibrary.FClamp` (- (`SceneCaptureComponent2D.FOVAngle` _scenecapturecomponent2d) (`self.ZoomSpeed`)) 60.0 110.0) _scenecapturecomponent2d)))

(event `Key|MouseScrollDown`
  (params (Key :type "Key Structure"))
  (bind _scenecapturecomponent2d (`self.SceneCaptureComponent2D`))
  ;[1 1 1] Scale
  (:`Pressed`
    (set `SceneCaptureComponent2D.FOVAngle` (`KismetMathLibrary.FClamp` (+ (`SceneCaptureComponent2D.FOVAngle` _scenecapturecomponent2d) (`self.ZoomSpeed`)) 60.0 110.0) _scenecapturecomponent2d)))

(fn `UserConstructionScript`)