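; BP_CarlAI is an AI-driven character, Carl, that follows the player while its Active flag is set.
; Each Tick calls FollowPlayer, which issues AI Move To targeting the player controller and calls itself again on success.
; While active, the player's AllowStand flag shows Carl with capsule collision, otherwise he is hidden with mesh and capsule collision off.
; The node restoring mesh collision is unconnected, so that collision is never re-enabled here.
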(event `self.ReceiveBeginPlay`)

(event `self.ReceiveTick`
  (params (DeltaSeconds :type "Float (single-precision)"))
  (bind _capsulecomponent (`self.CapsuleComponent`))
  (if (`self.Active`)
    (`self.Follow Player`)
    (if (`IncompleteEvolutionCharacter.AllowStand` (`self.Player`))
      (`self.SetActorHiddenInGame` false)
      (`PrimitiveComponent.SetCollisionEnabled` _capsulecomponent "QueryAndPhysics")
      (else
        (`self.SetActorHiddenInGame` true)
        (`PrimitiveComponent.SetCollisionEnabled` (`self.Mesh`) "NoCollision")
        (`PrimitiveComponent.SetCollisionEnabled` _capsulecomponent "NoCollision")))))

(event `Follow Player`
  (`|AIMoveTo` self (0.0 0.0 0.0) (`GameplayStatics.GetPlayerController` 0) 100.0
    (:`OnSuccess`
      (`self.Follow Player`))))

(fn `UserConstructionScript`)