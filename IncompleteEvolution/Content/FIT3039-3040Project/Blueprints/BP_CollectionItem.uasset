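; BP_CollectionItem is a collectible item that the first-person player can interact with to view it in a display.
; Its sphere overlap shows or hides a CollectionInteract_UI widget, creating a new instance each time, and trace checks toggle that widget's border opacity.
; Interact spawns a BP_CollectionDisplay at a far-off location and passes it the player, item mesh, name and description.
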(event `self.Sphere.OnComponentBeginOverlap`
  (params (OverlappedComponent :type "PrimitiveComponent Object Reference") (OtherActor :type "Actor Object Reference") (OtherComp :type "PrimitiveComponent Object Reference") (OtherBodyIndex :type Integer) (bFromSweep :type Boolean) (SweepResult :type "HitResult Structure (by ref)"))
  (bind _widget (`self.Widget`))
  (cast `/Game/FirstPerson/Blueprints/BP_FirstPersonCharacter` OtherActor)
  (bind _returnvalue (`|CreateWidget` "/Game/FIT3039-3040Project/UI/CollectionInteract_UI.CollectionInteract_UI_C"))
  (bind _output_get (set `self.Interaction Widget` _returnvalue))
  (`WidgetComponent.SetWidget` _widget _output_get)
  (`SceneComponent.SetVisibility` _widget true false))

(event `self.Sphere.OnComponentEndOverlap`
  (params (OverlappedComponent :type "PrimitiveComponent Object Reference") (OtherActor :type "Actor Object Reference") (OtherComp :type "PrimitiveComponent Object Reference") (OtherBodyIndex :type Integer))
  (cast `/Game/FirstPerson/Blueprints/BP_FirstPersonCharacter` OtherActor)
  (bind _returnvalue (`|CreateWidget` "/Game/FIT3039-3040Project/UI/CollectionInteract_UI.CollectionInteract_UI_C"))
  (set `self.Interaction Widget` _returnvalue)
  (`SceneComponent.SetVisibility` (`self.Widget`) false false))

(event `/Game/FIT3039-3040Project/Blueprints/BP_CollectionInterface.CanRecieveTrace`
  (params (CanInteract :type Boolean))
  (if CanInteract
    (bind _interaction_widget (`self.Interaction Widget`)
      (:`then`
        (`Widget.SetRenderOpacity` (`/Game/FIT3039-3040Project/UI/CollectionInteract_UI.InteractionBorder` _interaction_widget) 1.0))
      (:`else`))
    (else
      (bind _interaction_widget_2 (`self.Interaction Widget`)
        (:`then`
          (`Widget.SetRenderOpacity` (`/Game/FIT3039-3040Project/UI/CollectionInteract_UI.InteractionBorder` _interaction_widget_2) 0.0))
        (:`else`)))))

(event `/Game/FIT3039-3040Project/Blueprints/BP_CollectionInterface.Interact`
  (params (Player :type "/Game/FirstPerson/Blueprints/BP_FirstPersonCharacter Object Reference"))
  (bind _returnvalue (`|SpawnActorFromClass` "/Game/FIT3039-3040Project/Blueprints/BP_CollectionDisplay.BP_CollectionDisplay_C" (`KismetMathLibrary.MakeTransform` (10000000.0 10000000.0 10000000.0)) "Undefined" "OverrideRootScale" null null))
  (message `/Game/FIT3039-3040Project/Blueprints/BP_CollectionInterface.Display` _returnvalue Player (`StaticMeshComponent.StaticMesh` (`self.CollectionItem`)) (`self.CollectionName`) (`self.CollectionDescription`)))

(fn `UserConstructionScript`)